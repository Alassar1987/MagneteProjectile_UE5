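; Positive half of a magnet ammo pair, which finds its Minus counterpart and pulls it toward itself.
; Tick can grow a magnetic sensor sphere up to a maximum; overlapping the assigned MagnetPair destroys it and creates a two-point spline with a spline mesh link.
; After a delay, Tick stretches the link to the partner and applies a distance-scaled physics force to it, destroying the mesh if the partner becomes invalid.
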(event OnComponentBeginOverlap(MagneticSencsor)
  (params (OverlappedComponent :type Primitive%20Component%20Object%20Reference) (OtherActor :type Actor%20Object%20Reference) (OtherComp :type Primitive%20Component%20Object%20Reference) (OtherBodyIndex :type Integer) (bFromSweep :type Boolean) (SweepResult :type Hit%20Result%20Structure%20%28by%20ref%29))
  ;[1 1 1] Search for pair projectile
  (bind _asbp_magnet_ammo_minus (Utilities|Casting|CastToBP_MagnetAmmo_Minus OtherActor))
  (Variables|/Game/Magnet/BP_MagnetAmmo_Minus.BP_MagnetAmmo_Minus_C|SetRef_MagnetPlus _asbp_magnet_ammo_minus self)
  (if (== OtherActor (Variables|Calculated|GetMagnetPair))
    (Utilities|FlowControl|DoOnce false
      (:Completed
        ;[1 1 1] Calculating spline coordinates
        (Spline|AddSplinePoint (Variables|Default|GetSpline_String) (Transformation|GetActorLocation OtherActor) "World" true)
        (Components|DestroyComponent (Variables|Default|GetMagneticSencsor))
        (bind _returnvalue (AddComponent|AddSplineMeshComponent true))
        (SplineMesh|SetForwardAxis _returnvalue "Z" true)
        ;[1 1 1] Delay to attract
        (Utilities|FlowControl|Delay (Variables|Default|GetDraggingDelay))
        (Variables|Calculated|SetStartDrag true)))))

(event EventBeginPlay
  (|CallParentFunction))

(event EventTick
  (params (DeltaSeconds :type Float%20%28single-precision%29))
  (bind _spline_string (Variables|Default|GetSpline_String))
  (bind _magneticsencsor (Variables|Default|GetMagneticSencsor))
  (bind _sphereradius (Variables|/Script/Engine.SphereComponent|GetSphereRadius _magneticsencsor))
  (|CallParentFunction DeltaSeconds)
  (Utilities|FlowControl|Sequence
    (:then_0
      ;[1 1 1] Increasing Magnetic Sensor logic
      (Utilities|IsValid (stale OnComponentBeginOverlap(MagneticSencsor) OtherActor)
        (:Is%20Valid
          (if (== (Spline|GetNumberOfSplinePoints (Variables|Default|GetSpline_String)) 1)
            (Utilities|IsValid _magneticsencsor
              (:Is%20Valid
                (if (not (>= _sphereradius (Variables|Default|GetMaxMagneticSensorRadius)))
                  (Components|Sphere|SetSphereRadius _magneticsencsor (+ _sphereradius 5.0) true))))))))
    (:then_1
      (if (Variables|Calculated|GetStartDrag)
        (Utilities|FlowControl|Sequence
          (:then_0
            ;[1 1 1] Updating the final spline coordinate
            (Utilities|IsValid (stale OnComponentBeginOverlap(MagneticSencsor) OtherActor)
              (:Is%20Valid
                (if (== (Spline|GetNumberOfSplinePoints (Variables|Default|GetSpline_String)) 2)
                  (Spline|SetLocationatSplinePoint (Variables|Default|GetSpline_String) 1 (Transformation|GetActorLocation (stale OnComponentBeginOverlap(MagneticSencsor) OtherActor)) "World" true)
                  (SplineMesh|SetStartandEnd (stale OnComponentBeginOverlap(MagneticSencsor) _returnvalue) (Spline|GetLocationatSplinePoint _spline_string 0 "World") (Spline|GetTangentatSplinePoint _spline_string 0 "World") (Spline|GetLocationatSplinePoint _spline_string 1 "World") (Spline|GetTangentatSplinePoint _spline_string 1 "World") true :!class /Script/Engine.SplineMeshComponent)))
              (:Is%20Not%20Valid
                (Utilities|IsValid (stale OnComponentBeginOverlap(MagneticSencsor) _returnvalue)
                  (:Is%20Valid
                    ;[1 1 1] Destroy spline mesh if the pair connection is lost
                    (Components|DestroyComponent (stale OnComponentBeginOverlap(MagneticSencsor) _returnvalue)))))))
          (:then_1
            ;[1 1 1] Attracting pair
            (Utilities|IsValid (stale OnComponentBeginOverlap(MagneticSencsor) _asbp_magnet_ammo_minus)
              (:Is%20Valid
                (Variables|Default|SetDragForceEffective 0.0)
                (Physics|SetSimulatePhysics (Variables|/Game/Magnet/BaseMagnetAmmo.BaseMagnetAmmo_C|GetCollisionSphere (stale OnComponentBeginOverlap(MagneticSencsor) _asbp_magnet_ammo_minus)) true)
                (Physics|AddForce (Variables|/Game/Magnet/BaseMagnetAmmo.BaseMagnetAmmo_C|GetCollisionSphere (stale OnComponentBeginOverlap(MagneticSencsor) _asbp_magnet_ammo_minus)) (/ (* (- (Transformation|GetWorldLocation (Variables|Default|GetCollisionSphere)) (Transformation|GetWorldLocation (Variables|/Game/Magnet/BaseMagnetAmmo.BaseMagnetAmmo_C|GetCollisionSphere (stale OnComponentBeginOverlap(MagneticSencsor) _asbp_magnet_ammo_minus)))) (Variables|Default|GetDragForceMax)) 2.0) "None" false)))))))))

(fn ConstructionScript
  (|CallParentFunction))