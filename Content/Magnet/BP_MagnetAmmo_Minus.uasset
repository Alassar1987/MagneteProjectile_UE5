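; BP_MagnetAmmo_Minus is the negative half of a magnet projectile pair, pulling its plus counterpart toward itself.
; Each Tick, when RefMagnetPlus is valid and its StartDrag flag is set, it enables physics on that projectile's collision sphere.
; It then applies a force along the vector between the two spheres, scaled by half of DragForceMax, so pull grows with distance.
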(event EventBeginPlay
  (|CallParentFunction))

(event Collision|EventActorBeginOverlap
  (params (OtherActor :type Actor%20Object%20Reference))
  (|CallParentFunction OtherActor))

(event EventTick
  (params (DeltaSeconds :type Float%20%28single-precision%29))
  (bind _ref_magnetplus (Variables|Calculated|GetRef_MagnetPlus))
  (bind _collisionsphere (Variables|/Game/Magnet/BaseMagnetAmmo.BaseMagnetAmmo_C|GetCollisionSphere _ref_magnetplus))
  (|CallParentFunction DeltaSeconds)
  ;[1 1 1] Projectile attracts it's pair
  (Utilities|IsValid _ref_magnetplus
    (:Is%20Valid
      (if (Variables|/Game/Magnet/BP_MagnetAmmo_Plus.BP_MagnetAmmo_Plus_C|GetStartDrag _ref_magnetplus)
        (Physics|SetSimulatePhysics _collisionsphere true)
        (Physics|AddForce _collisionsphere (/ (* (- (Transformation|GetWorldLocation (Variables|Default|GetCollisionSphere)) (Transformation|GetWorldLocation _collisionsphere)) (Variables|Default|GetDragForceMax)) 2.0) "None" false)))))

(fn ConstructionScript
  (|CallParentFunction))